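; Zombie enemy for the runner game that moves toward the player and cuts Runner_Character health when its box is overlapped.
; A fast looping timer drives movement and facing within a Y range, changes direction while the player's shield is active, and destroys zombies left too far behind.
; A slower timer refreshes the runner reference and checks Dead.
; Death disables collision and destroys the actor after a delay, with DirectDeath adding a dying animation.
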(event `self.Box.OnComponentBeginOverlap`
  (params (OverlappedComponent :type "PrimitiveComponent Object Reference") (OtherActor :type "Actor Object Reference") (OtherComp :type "PrimitiveComponent Object Reference") (OtherBodyIndex :type Integer) (bFromSweep :type Boolean) (SweepResult :type "HitResult Structure (by ref)"))
  ;[1 1 1] Attack
  (bind _asrunner_character (cast `/Game/BluePrints/Runner_Character` OtherActor))
  (set `self.AttackZombie1` true)
  (if (not (`self.Dead`))
    (set `/Game/BluePrints/Runner_Character.Health` (- (`/Game/BluePrints/Runner_Character.Health` _asrunner_character) 0.5) _asrunner_character)))

(event `Distance`
  ;[1 1 1] DeathCheck
  (if (`self.Dead`)
    (`PrimitiveComponent.SetCollisionEnabled` (`self.CapsuleComponent`) "NoCollision" :!label _label)
    (`PrimitiveComponent.SetCollisionEnabled` (`self.Box`) "NoCollision")
    (`KismetSystemLibrary.Delay` 3.0)
    (`self.K2_DestroyActor`)))

(event `DirectDeath`
  ;[1 1 1] DeathCheck
  (`/Engine/EditorBlueprintResources/StandardMacros.DoOnce` false
    (:`Completed`
      (`SkeletalMeshComponent.PlayAnimation` (`self.Mesh`) "/Game/Zombie/Zombie2/Animation/Zombie_Dying.Zombie_Dying" false)
      (goto _label))))

(event `self.Box.OnComponentEndOverlap`
  (params (OverlappedComponent :type "PrimitiveComponent Object Reference") (OtherActor :type "Actor Object Reference") (OtherComp :type "PrimitiveComponent Object Reference") (OtherBodyIndex :type Integer))
  ;[1 1 1] Attack
  (cast `/Game/BluePrints/Runner_Character` OtherActor)
  (set `self.AttackZombie1` false))

(event `Walk`
  ;[1 1 1] Timer
  (`KismetSystemLibrary.K2_SetTimerDelegate` (delegate `Timer`) 0.02 true))

(event `DistanceCheck`
  (bind _returnvalue (`GameplayStatics.GetPlayerCharacter` 0))
  (bind _returnvalue_2 (`GameplayStatics.GetPlayerCharacter` 0))
  (bind (_returnvalue_x _returnvalue_y) (`KismetMathLibrary.BreakVector` (`self.K2_GetActorLocation`)))
  (bind _returnvalue_3 (`self.K2_GetActorLocation`))
  (bind _returnvalue_4 (`GameplayStatics.GetPlayerCharacter` 0))
  (bind (_returnvalue_x_2 _returnvalue_y_2) (`KismetMathLibrary.BreakVector` (`self.K2_GetActorLocation`)))
  (bind _returnvalue_5 (`self.K2_GetActorLocation` _returnvalue))
  (bind (_returnvalue_x_3 _returnvalue_y_3) (`KismetMathLibrary.BreakVector` (`self.K2_GetActorLocation` _returnvalue_2)))
  (bind (_returnvalue_x_4 _returnvalue_y_4) (`KismetMathLibrary.BreakVector` (`self.K2_GetActorLocation` _returnvalue_4)))
  (bind _returnvalue_6 (- _returnvalue_y_4 _returnvalue_y_2))
  (bind _returnvalue_7 (- _returnvalue_y_3 _returnvalue_y))
  ;[1 1 1] Inrange
  (`/Engine/EditorBlueprintResources/StandardMacros.IsValid` _returnvalue_4
    (:`Is Valid`
      (if (not (>= _returnvalue_6 1000.0))
        (if (not (< _returnvalue_6 -5000.0))
          ;[1 1 1] Distance Between Players
          (`/Engine/EditorBlueprintResources/StandardMacros.IsValid` _returnvalue
            (:`Is Valid`
              (if (`/Game/BluePrints/Runner_Character.ShieldAvctivated` (`self.RunnerCharRef`))
                (`self.K2_AddActorLocalOffset` (* (`KismetMathLibrary.Normal` (+ _returnvalue_5 _returnvalue_3)) (`self.speed`)))
                ;[1 1 1] Rotation
                (`/Engine/EditorBlueprintResources/StandardMacros.CompareFloat` _returnvalue_7
                  (:`>`
                    (`SceneComponent.K2_SetWorldRotation` (`self.Mesh`) (struct :`Yaw` 180.0) false false :!label _label_2))
                  (:`<`
                    (`SceneComponent.K2_SetWorldRotation` :`self` (`self.Mesh`) :!label _label_3)))
                (else
                  (`self.K2_AddActorLocalOffset` (* (`KismetMathLibrary.Normal` (- _returnvalue_5 _returnvalue_3)) (`self.speed`)))
                  (`/Engine/EditorBlueprintResources/StandardMacros.IsValid` _returnvalue_2
                    (:`Is Valid`
                      (`/Engine/EditorBlueprintResources/StandardMacros.CompareFloat` _returnvalue_7
                        (:`>`
                          (goto _label_3))
                        (:`<`
                          (goto _label_2))))))))))
        (else
          (`self.K2_DestroyActor`))))))

(event `self.ReceiveBeginPlay`
  ;[1 1 1] Timer
  (`|ExecutionSequence`
    (:`then_0`
      (`self.Walk`))
    (:`then_1`
      (`KismetSystemLibrary.K2_SetTimerDelegate` (delegate `Timer2`) 0.5 true))))

(event `Timer`
  ;[1 1 1] Timer
  (`self.DistanceCheck`))

(event `Timer2`
  ;[1 1 1] Timer
  (`|ExecutionSequence`
    (:`then_0`
      (`self.Distance`))
    (:`then_1`
      (bind _returnvalue (`GameplayStatics.GetActorOfClass` "/Game/BluePrints/Runner_Character.Runner_Character_C"))
      (set `self.RunnerCharRef` _returnvalue))))

(fn `UserConstructionScript`)