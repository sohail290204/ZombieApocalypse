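; Ground1 is a floor segment for a runner game that keeps the track going and cleans up behind the player.
; When Runner_Character enters the Spawner trigger, GameMode3d spawns a new floor and coins; two seconds after leaving, the segment destroys itself.
; On BeginPlay it switches child spotlights tagged "Lights" on or off from the game instance's Evening flag, and starts a looping timer that caches the game mode.
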(event `Ref`
  (`KismetSystemLibrary.K2_SetTimerDelegate` (delegate `Event Tick`) 1.0 true))

(event `Event Tick`
  (bind _asgame_mode_3d (cast `/Game/GameMode/GameMode3d` (`GameplayStatics.GetGameMode`))))

(event `self.Spawner.OnComponentBeginOverlap`
  (params (OverlappedComponent :type "PrimitiveComponent Object Reference") (OtherActor :type "Actor Object Reference") (OtherComp :type "PrimitiveComponent Object Reference") (OtherBodyIndex :type Integer) (bFromSweep :type Boolean) (SweepResult :type "HitResult Structure (by ref)"))
  (cast `/Game/BluePrints/Runner_Character` OtherActor)
  (`/Game/GameMode/GameMode3d.SpawnFloor` (stale `Event Tick` _asgame_mode_3d))
  (`/Game/GameMode/GameMode3d.Coins` (stale `Event Tick` _asgame_mode_3d)))

(event `self.Spawner.OnComponentEndOverlap`
  (params (OverlappedComponent :type "PrimitiveComponent Object Reference") (OtherActor :type "Actor Object Reference") (OtherComp :type "PrimitiveComponent Object Reference") (OtherBodyIndex :type Integer))
  (cast `/Game/BluePrints/Runner_Character` OtherActor)
  (`KismetSystemLibrary.Delay` 2.0)
  (`self.K2_DestroyActor`))

(event `self.ReceiveBeginPlay`
  (`self.Ref`)
  (bind _aszombei_game_instance (cast `/Game/ZombeiGameInstance` (`GameplayStatics.GetGameInstance`)))
  (if (`/Game/ZombeiGameInstance.Evening` _aszombei_game_instance)
    (for _array_element (`SceneComponent.GetChildrenComponents` (`self.DefaultSceneRoot`) true)
      (if (`ActorComponent.ComponentHasTag` _array_element "Lights")
        (bind _asspot_light_component (cast `SpotLightComponent` _array_element))
        (`LightComponent.SetIntensity` _asspot_light_component 40000.0)))
    (else
      (for _array_element_2 (`SceneComponent.GetChildrenComponents` (`self.DefaultSceneRoot`) true)
        (if (`ActorComponent.ComponentHasTag` _array_element_2 "Lights")
          (bind _asspot_light_component_2 (cast `SpotLightComponent` _array_element_2))
          (`LightComponent.SetIntensity` _asspot_light_component_2 0.0))))))

(fn `UserConstructionScript`)